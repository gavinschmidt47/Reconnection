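; BP_GridFloorSector is a floor sector actor that works out its own cell coordinate on a grid.
; On BeginPlay it divides the Box component's bounds origin in X and Y by the Cube's world scale times 100, treating the scaled cube as the cell size.
; The rounded results are stored in GridPosition with Z at zero.
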(event EventBeginPlay
  (bind _cube (Variables|Default|GetCube))
  (bind _box (Variables|Default|GetBox))
  (bind _origin (Collision|GetComponentBounds _box))
  (bind _returnvalue (Transformation|GetWorldScale _cube))
  (Variables|Default|SetGridPosition (Math|Vector|MakeVector (Math|Conversions|ToFloat(Integer) (Class|KismetMathLibrary|Round64 (/ (.x _origin) (* (.x _returnvalue) 1e+02)))) (Math|Conversions|ToFloat(Integer) (Class|KismetMathLibrary|Round64 (/ (.y _origin) (* (.y _returnvalue) 1e+02)))) 0.0)))

(event Collision|EventActorBeginOverlap
  (params (OtherActor :type Actor%20Object%20Reference)))

(event EventTick
  (params (DeltaSeconds :type Float%20%28single-precision%29)))

(fn ConstructionScript)