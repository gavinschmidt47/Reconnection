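; BP_HighLevelEnemyActions is the decision logic that picks a high-level enemy's action in turn-based combat.
; ChooseAction heals at or below half health; otherwise it attacks through its BP_General owner if the last damage received does not exceed the last damage sent, and blocks if it does.
; Damage and SendDamage record those two values, and each completed action calls StartingNextTurn.
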(event EventDamage
  (params (Damage :type Float%20%28single-precision%29))
  (bind _output_get (Variables|Default|SetLastDamageReceive Damage)))

(event EventSendDamage
  (params (Damage :type Float%20%28single-precision%29) (Target :type Fighter%20Object%20Reference))
  (bind _output_get (Variables|Default|SetLastDamageSent Damage)))

(event EventChooseAction
  (bind _output_get (Variables|Default|SetCriticalHealth (<= (Variables|Default|GetCurrentHealth) (/ (Variables|Default|GetMaxHealth) 2.0))))
  (if _output_get
    (Class|Fighter|CallHeal)
    (elif (<= (stale EventDamage _output_get) (stale EventSendDamage _output_get))
      (bind _asbp_general (Utilities|Casting|CastToBP_General (Components|GetOwner)))
      (Default|AttackPlayer _asbp_general)
      (else
        (Class|Fighter|CallBlock))))
  (Default|CallStartingNextTurn))

(fn ConstructionScript)