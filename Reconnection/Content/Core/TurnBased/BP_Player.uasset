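; BP_Player is the player's camera pawn for grid-based, turn-based play, with movement, zoom, middle-mouse rotation and a downward trace that holds its height above the ground.
; On BeginPlay it spawns a party actor and a ghost mover.
; Left clicks multi-trace under the cursor to target a grid sector's enemy or send the ghost along a path.
; The party AI-moves to the ghost's endpoint if the spaces moved are within MaxMovement.
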(event Input|EnhancedActionEvents|EnhancedInputActionZoomAction
  (params (ActionValue :type Float%20%28double-precision%29) (ElapsedSeconds :type Float%20%28double-precision%29) (TriggeredSeconds :type Float%20%28double-precision%29) (InputAction :type Input%20Action%20Object%20Reference :default "/Game/Core/TopDown/NewCamera/Input/Actions/ZoomAction.ZoomAction"))
  (Variables|/Script/Engine.SpringArmComponent|SetTargetArmLength (Variables|Default|GetSpringArm) (Math|Float|Clamp(Float) (+ (Variables|/Script/Engine.SpringArmComponent|GetTargetArmLength (Variables|Default|GetSpringArm)) (* ActionValue 5e+01)) 2.5e+02 1e+03)))

(event Input|EnhancedActionEvents|EnhancedInputActionRotationAction
  (params (ActionValue :type Vector%202D%20Structure) (ElapsedSeconds :type Float%20%28double-precision%29) (TriggeredSeconds :type Float%20%28double-precision%29) (InputAction :type Input%20Action%20Object%20Reference :default "/Game/Core/TopDown/NewCamera/Input/Actions/RotationAction.RotationAction"))
  (bind _returnvalue (Transformation|GetActorRotation))
  (bind (_roll _pitch _yaw) (Math|Rotator|BreakRotator _returnvalue))
  (if (Variables|Default|GetRotationActivate)
    (Transformation|SetActorRotation (Math|Rotator|MakeRotator 0.0 _pitch (Math|Float|Clamp(Float) (+ _yaw (.X (Math|Vector2D|BreakVector2D ActionValue))) -3.6e+02 3.6e+02)))))

(event Input|EnhancedActionEvents|EnhancedInputActionMoveAction
  (params (ActionValue :type Vector%202D%20Structure) (ElapsedSeconds :type Float%20%28double-precision%29) (TriggeredSeconds :type Float%20%28double-precision%29) (InputAction :type Input%20Action%20Object%20Reference :default "/Game/Core/TopDown/NewCamera/Input/Actions/MoveAction.MoveAction"))
  (bind (_x _y) (Math|Vector2D|BreakVector2D ActionValue))
  (Development|PrintString (Utilities|String|ToString(Vector2d) ActionValue))
  (Pawn|Input|AddMovementInput (Transformation|GetActorForwardVector) _x false)
  (Pawn|Input|AddMovementInput (Transformation|GetActorRightVector) _y false))

(event EventBeginPlay
  (bind _returnvalue (Game|GetPlayerController 0))
  (bind _returnvalue_2 (Game|SpawnActorfromClass "/Game/Core/TurnBased/BP_Party.BP_Party_C" (Transformation|GetWorldTransform (Variables|Default|GetDefaultSceneRoot)) "AlwaysSpawn" "MultiplyWithRoot" 0 0))
  (bind _output_get (Variables|Default|SetParty _returnvalue_2))
  (bind _returnvalue_3 (Game|SpawnActorfromClass "/Game/Core/TurnBased/BP_GhostMove.BP_GhostMove_C" (Transformation|GetActorTransform _output_get) "AlwaysSpawn" "OverrideRootScale" 0 0))
  (Variables|Default|SetGhostMover _returnvalue_3)
  (Development|PrintString "Spawned Ghost")
  (Variables|/Script/Engine.PlayerController|SetbEnableClickEvents _returnvalue true)
  (Variables|/Script/Engine.PlayerController|SetbEnableMouseOverEvents _returnvalue true)
  (Variables|/Script/Engine.PlayerController|SetbShowMouseCursor _returnvalue true))

(event EventTick
  (params (DeltaSeconds :type Float%20%28single-precision%29))
  (bind _returnvalue (Transformation|GetActorLocation))
  (bind _returnvalue_2 (Transformation|GetActorLocation))
  (bind _returnvalue_3 (Transformation|GetActorLocation))
  (bind _outhit (Collision|LineTraceByChannel (Math|Vector|MakeVector (.x _returnvalue_2) (.y _returnvalue_2) (+ (.z _returnvalue_2) (Variables|Default|GetDesireOffset))) (Math|Vector|MakeVector (.x _returnvalue) (.y _returnvalue) (+ (.z _returnvalue) -1e+03)) "TraceTypeQuery1" false 0 "ForDuration"))
  (Transformation|SetActorLocation (Math|Vector|MakeVector (.x _returnvalue_3) (.y _returnvalue_3) (+ (.Z (Math|Vector|BreakVector (.ImpactPoint (Collision|BreakHitResult _outhit)))) (Variables|Default|GetDesireOffset))) false false))

(event Input|MouseEvents|MiddleMouseButton
  (params (Key :type Key%20Structure))
  (:Pressed
    (Variables|Default|SetRotationActivate true))
  (:Released
    (Variables|Default|SetRotationActivate false)))

(event Input|MouseEvents|LeftMouseButton
  (params (Key :type Key%20Structure))
  (bind _returnvalue (Game|GetPlayerController 0))
  (bind (_worldlocation _worlddirection) (Game|Player|ConvertMouseLocationToWorldSpace _returnvalue))
  (:Pressed
    (Development|PrintString "Click")
    (bind (_outhits _returnvalue_2) (Collision|MultiLineTraceByChannel _worldlocation (+ _worldlocation (* _worlddirection (Variables|Default|GetMaxMouseRaycast))) "TraceTypeQuery1" true 0 "Persistent"))
    (if _returnvalue_2
      (for _array_element _outhits
        (|HandleClicks (.hitactor _array_element)))
      (else
        (Development|PrintString "No hit")))))

(fn ConstructionScript)

(event Custom|CanPlayerMove
  (params (SpacesMoved :type Integer) (CurrentLocation :type Vector))
  (Math|Integer|CompareInt SpacesMoved (Math|Float|Truncate (Variables|/Script/Reconnection.Fighter|GetMaxMovement (Variables|Default|GetBP_PlayerActions)))
    (:==
      _)
    (:<
      _))
  (AI|AIMoveTo (Variables|Default|GetParty) CurrentLocation 0 5.0 false))