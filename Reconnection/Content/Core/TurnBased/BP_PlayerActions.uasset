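; BP_PlayerActions handles the player's turn-based actions: block, heal and damage.
; Block and Heal derive damage reduction and health gain from a score offset by 50 plus buff and base values, then start the next turn.
; SendDamage subtracts from a temporary General health value, then either broadcasts the attack and advances the turn or, at zero or below, signals death.
; Heal's broadcast amount omits the score term.
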(event EventHeal
  (bind _baseheal (Variables|Default|GetBaseHeal))
  (bind _healbuff (Variables|Default|GetHealBuff))
  (Variables|Default|SetCurrentHealth (+ (- (Variables|Default|GetHealScore) 50) (Variables|Default|GetCurrentHealth) _healbuff _baseheal))
  (Default|CallHealing (+ _healbuff _baseheal))
  (Default|CallStartNextTurn))

(event EventSendDamage
  (params (Damage :type Float%20%28single-precision%29) (Target :type Fighter%20Object%20Reference))
  (bind _output_get (Variables|Default|SetGeneralHealthTemp (- (Variables|Default|GetGeneralHealthTemp) Damage)))
  (Math|Float|CompareFloat _output_get 0.0
    (:>
      (Development|PrintString (Utilities|String|ToString(Float) Damage))
      (Development|PrintString (Utilities|String|ToString(Float) _output_get))
      (Default|CallAttacking Damage)
      (Default|CallStartNextTurn))
    (:==
      (Default|CallTempGenDeath :!label _label))
    (:<
      (goto _label))))

(event EventBlock
  (Variables|Default|SetDamageReduction (+ (- (Variables|Default|GetTankScore) 50) (Variables|Default|GetBlockBuff) (Variables|Default|GetBaseBlock)))
  (Default|CallStartNextTurn))

(fn ConstructionScript)