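; Enemy component for turn-based combat that decides between attacking the player's BP_PlayerActions component and healing itself.
; BeginPlay caches that component after a short delay.
; ChooseAction acts only at or below half health, using a health-scaled random roll that favors healing as health drops; above half, nothing is wired.
; Damage events record the last damage received and sent, but the comparison between them is unused.
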(event EventDamage
  (params (Damage :type Float%20%28single-precision%29))
  (bind _output_get (Variables|Default|SetLastDamageReceive Damage)))

(event EventSendDamage
  (params (Damage :type Float%20%28single-precision%29) (Target :type Fighter%20Object%20Reference))
  (bind _output_get (Variables|Default|SetLastDamageSent Damage)))

(event EventChooseAction
  (bind _currenthealth (Variables|Default|GetCurrentHealth))
  (bind _maxhealth (Variables|Default|GetMaxHealth))
  (bind _returnvalue (/ _maxhealth 2.0))
  (bind _output_get (Variables|Default|SetCriticalHealth (<= _currenthealth _returnvalue)))
  (if _output_get
    (Math|Float|CompareFloat (Math|Random|RandomFloatinRange 0.0 (/ _currenthealth _returnvalue)) 0.5
      (:>
        (Class|Fighter|Attack (Variables|Default|GetPlayerFighterComp) :!label _label))
      (:==
        (goto _label))
      (:<
        (Class|Fighter|Heal)))))

(event EventBeginPlay
  (Utilities|FlowControl|Delay 0.2)
  (bind _returnvalue (Actor|GetActorOfClass "/Game/Core/TurnBased/BP_Player.BP_Player_C"))
  (Variables|Default|SetPlayerFighterComp (Actor|GetComponentbyClass _returnvalue "/Game/Core/TurnBased/BP_PlayerActions.BP_PlayerActions_C")))

(fn ConstructionScript)