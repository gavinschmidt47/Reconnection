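; BP_Enemy is a turn-based enemy that moves to a given destination and counts the grid spaces it touches.
; MoveEnemy resets the count and runs AIMoveTo; on success it calls the FinishPath dispatcher and clears IsMoving.
; Each overlap with a SpaceCol-tagged actor increments the count and sets the capsule material to Burnt below a threshold, otherwise M_Enemy.
; Debug prints report movement results and overlaps.
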(event Custom|MoveEnemy
  (params (GoalDestination :type Vector))
  (Variables|Default|SetTouchedSpace 0)
  (AI|AIMoveTo self GoalDestination 0 5.0 false
    (:then
      (Development|PrintString (Utilities|String|Append "Heading to " (Utilities|String|ToString(Vector) GoalDestination))))
    (:OnSuccess
      (Development|PrintString "Arrived")
      (Default|CallFinishPath)
      (Variables|Default|SetIsMoving false))
    (:OnFail
      (Development|PrintString "failed"))))

(event Collision|EventActorBeginOverlap
  (params (OtherActor :type Actor%20Object%20Reference))
  (if (Actor|ActorHasTag OtherActor "SpaceCol")
    (if true
      (bind _result (Math|Integer|IncrementInt (Variables|Default|GetTouchedSpace))
        (:%20%20
          (Development|PrintString (Utilities|String|ToString(Integer) _result))
          (Math|Integer|CompareInt _result 5
            (:>
              (Rendering|Material|SetMaterial (Variables|Collision|GetCapsuleComponent) 0 "/Game/Materials/M_Enemy.M_Enemy" :!label _label))
            (:==
              (goto _label))
            (:<
              (Rendering|Material|SetMaterial (Variables|Collision|GetCapsuleComponent) 0 "/Game/Materials/Burnt.Burnt"))))))
    (else
      (Development|PrintString (Utilities|GetDisplayName OtherActor)))))

(fn ConstructionScript)