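; BP_General is an actor in the turn-based system that links high-level enemy actions to the player's turn.
; On BeginPlay it finds BP_Player, caches its BP_PlayerActions component and binds to the StartingNextTurn dispatcher on BPHighLevelEnemyActions.
; When that dispatcher fires, it starts the player's turn.
; AttackPlayer passes the cached player component to the enemy Attack call, but nothing in this Blueprint calls it.
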(event Custom|StartingNextTurn
  (CallFunction|StartPlayerTurn))

(event EventBeginPlay
  (bind _returnvalue (Actor|GetActorOfClass "/Game/Core/TurnBased/BP_Player.BP_Player_C"))
  (Variables|Default|SetPlayer (Actor|GetComponentbyClass _returnvalue "/Game/Core/TurnBased/BP_PlayerActions.BP_PlayerActions_C"))
  (EventDispatchers|BindEventtoStartingNextTurn (Variables|Default|GetBP_HighLevelEnemyActions) (delegate Custom|StartingNextTurn)))

(event Collision|EventActorBeginOverlap
  (params (OtherActor :type Actor%20Object%20Reference)))

(event EventTick
  (params (DeltaSeconds :type Float%20%28single-precision%29)))

(fn ConstructionScript)

(fn AttackPlayer
  (Class|Fighter|Attack (Variables|Default|GetBP_HighLevelEnemyActions) (Variables|Default|GetPlayer)))

(fn StartPlayerTurn
  (Class|Fighter|StartTurn (Variables|Default|GetPlayer)))