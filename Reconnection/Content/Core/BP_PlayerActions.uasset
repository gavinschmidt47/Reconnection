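; BP_PlayerActions defines the player's Block and Heal actions, whose strength depends on opinion scores.
; On BeginPlay it casts player state 0 to BP_OpinionScores and caches it.
; Block sets DamageReduction from base, buff and TankOpinion's offset from a neutral 50.
; Heal adds the equivalent HealerOpinion-based amount to CurrentHealth, with no clamping in either action.
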(event EventHeal
  (Variables|Default|SetCurrentHealth (+ (- (Variables|/Game/Core/BP_OpinionScores.BP_OpinionScores_C|GetHealerOpinion (Variables|Default|GetAs%20BP%20Opinion%20Scores)) 50) (Variables|Default|GetCurrentHealth) (Variables|Default|GetHealBuff) (Variables|Default|GetBaseHeal))))

(event EventBeginPlay
  (bind _asbp_opinion_scores (Utilities|Casting|CastToBP_OpinionScores (Game|GetPlayerState 0)))
  (Variables|Default|SetAs%20BP%20Opinion%20Scores _asbp_opinion_scores))

(event EventBlock
  (Variables|Default|SetDamageReduction (+ (- (Variables|/Game/Core/BP_OpinionScores.BP_OpinionScores_C|GetTankOpinion (Variables|Default|GetAs%20BP%20Opinion%20Scores)) 50) (Variables|Default|GetBlockBuff) (Variables|Default|GetBaseBlock))))