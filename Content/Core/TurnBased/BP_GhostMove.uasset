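; Ghost pawn for turn-based movement that walks to a goal and counts the spaces it crosses.
; StartMove ignores requests while moving, otherwise reveals the ghost and runs AI MoveTo.
; Overlaps with SpaceCol-tagged actors increment the count and swap the capsule material around a five-space threshold.
; Arrival reports count and location through CallFinishPath; both success and failure hide and deactivate the ghost.
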(event Custom|CheckMove
  (params (GoalDestination :type Vector))
  (Rendering|SetActorHiddenInGame false)
  (Collision|SetActorEnableCollision true)
  (Actor|Tick|SetActorTickEnabled true)
  (Variables|Default|SetTouchedSpace 0)
  (AI|AIMoveTo self GoalDestination 0 5.0 false
    (:then
      (Development|PrintString (Utilities|String|Append "Heading to " (Utilities|String|ToString(Vector) GoalDestination))))
    (:OnSuccess
      (Development|PrintString "Arrived")
      (Default|CallFinishPath (Variables|Default|GetTouchedSpace) (Transformation|GetActorLocation))
      (Rendering|SetActorHiddenInGame true :!label _label)
      (Collision|SetActorEnableCollision false)
      (Actor|Tick|SetActorTickEnabled false)
      (Variables|Default|SetIsMoving false))
    (:OnFail
      (Development|PrintString "failed")
      (goto _label))))

(event Collision|EventActorBeginOverlap
  (params (OtherActor :type Actor%20Object%20Reference))
  (if (Actor|ActorHasTag OtherActor "SpaceCol")
    (if true
      (bind _result (Math|Integer|IncrementInt (Variables|Default|GetTouchedSpace))
        (:%20%20
          (Development|PrintString (Utilities|String|ToString(Integer) _result))
          (Math|Integer|CompareInt _result 5
            (:>
              (Rendering|Material|SetMaterial (Variables|Collision|GetCapsuleComponent) 0 "/Game/ArtSources/Materials/M_Enemy.M_Enemy" :!label _label))
            (:==
              (goto _label))
            (:<
              (Rendering|Material|SetMaterial (Variables|Collision|GetCapsuleComponent) 0 "/Game/ArtSources/Materials/Burnt.Burnt"))))))
    (else
      (Development|PrintString (Utilities|GetDisplayName OtherActor)))))

(fn ConstructionScript)

(fn StartMove
  (params (PlaceToGo :type Vector))
  (if (not (Variables|Default|GetIsMoving))
    (Variables|Default|SetIsMoving true)
    (CallFunction|CheckMove PlaceToGo)))